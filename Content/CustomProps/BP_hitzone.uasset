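; BP_hitzone is a one-time target that registers fireball hits toward a magic wall's hit count.
; When a BP_spell_fireball first overlaps its Hitzone component, it increments NumHits on the BP_Magicwall found through GetActorOfClass.
; It then clears its NotHit flag to ignore later hits and changes its point light's color to mark itself as hit.
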(event OnComponentBeginOverlap(hitzone)
  (params (OverlappedComponent :type Primitive%20Component%20Object%20Reference) (OtherActor :type Actor%20Object%20Reference) (OtherComp :type Primitive%20Component%20Object%20Reference) (OtherBodyIndex :type Integer) (bFromSweep :type Boolean) (SweepResult :type Hit%20Result%20Structure%20%28by%20ref%29))
  (Utilities|Casting|CastToBP_spell_fireball OtherActor)
  (if (Variables|Default|GetnotHit)
    (bind _returnvalue (Actor|GetActorOfClass "/Game/CustomProps/BP_Magicwall.BP_Magicwall_C"))
    (bind _result (Math|Integer|IncrementInt (Variables|/Game/CustomProps/BP_Magicwall.BP_Magicwall_C|GetNumHits _returnvalue))
      (:%20%20
        (Variables|/Game/CustomProps/BP_Magicwall.BP_Magicwall_C|SetNumHits _returnvalue _result)
        (Variables|Default|SetnotHit false)
        (Rendering|Components|Light|SetLightColor (Variables|Default|GetPointLight) (Variables|Default|GetNew%20Light%20Color) true)))))

(event EventBeginPlay)

(event Collision|EventActorBeginOverlap
  (params (OtherActor :type Actor%20Object%20Reference)))

(event EventTick
  (params (DeltaSeconds :type Float%20%28single-precision%29)))

(fn ConstructionScript)