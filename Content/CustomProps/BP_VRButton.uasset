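; BP_VRButton is a physical VR push button that permanently opens the final gate when a VRPawn touches it.
; Box overlap slides the Button component inward, and ending the overlap slides it back to the position cached at BeginPlay.
; The first press recolors the PointLight and destroys the BP_finalGate actor found by class, with the Activate flag blocking repeat triggers.
; The original light color is cached but never restored.
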(event OnComponentBeginOverlap(Box)
  (params (OverlappedComponent :type Primitive%20Component%20Object%20Reference) (OtherActor :type Actor%20Object%20Reference) (OtherComp :type Primitive%20Component%20Object%20Reference) (OtherBodyIndex :type Integer) (bFromSweep :type Boolean) (SweepResult :type Hit%20Result%20Structure%20%28by%20ref%29))
  (Utilities|Casting|CastToVRPawn OtherActor)
  (Components|MoveComponentTo (Variables|Default|GetButton) (- (Variables|Default|GetButtonStart) "0.000000,5.000000,0.000000") "0, 0, 0" false false 0.1 false)
  (CallFunction|ButtonActivate))

(event OnComponentEndOverlap(Box)
  (params (OverlappedComponent :type Primitive%20Component%20Object%20Reference) (OtherActor :type Actor%20Object%20Reference) (OtherComp :type Primitive%20Component%20Object%20Reference) (OtherBodyIndex :type Integer))
  (Utilities|Casting|CastToVRPawn OtherActor)
  (Components|MoveComponentTo (Variables|Default|GetButton) (Variables|Default|GetButtonStart) "0, 0, 0" false false 0.1 false))

(event Custom|ButtonActivate
  (if (not (Variables|Default|GetActivate))
    (Rendering|Components|Light|SetLightColor (Variables|Default|GetPointLight) (Variables|Default|GetButtonActiveColor) true)
    (Variables|Default|SetActivate true)
    (bind _returnvalue (Actor|GetActorOfClass "/Game/CustomProps/BP_finalGate.BP_finalGate_C"))
    (Actor|DestroyActor _returnvalue)))

(event EventBeginPlay
  (Variables|Default|SetButtonStart (Variables|/Script/Engine.SceneComponent|GetRelativeLocation (Variables|Default|GetButton)))
  (Variables|Default|SetButtonDeactivateColor (Rendering|Components|Light|GetLightColor (Variables|Default|GetPointLight))))

(fn ConstructionScript)