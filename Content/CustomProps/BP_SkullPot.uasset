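; BP_SkullPot is a VR prop that detects skulls placed in its trigger box and lights up in response.
; A BP_skull entering or leaving the Box raises or lowers SkullNums on the player's VRPawn and sets the Active flag.
; That flag switches the PointLight between ActiveColor and its original color, cached at BeginPlay.
; Active is a simple boolean, so any skull leaving turns it off.
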(event OnComponentBeginOverlap(Box)
  (params (OverlappedComponent :type Primitive%20Component%20Object%20Reference) (OtherActor :type Actor%20Object%20Reference) (OtherComp :type Primitive%20Component%20Object%20Reference) (OtherBodyIndex :type Integer) (bFromSweep :type Boolean) (SweepResult :type Hit%20Result%20Structure%20%28by%20ref%29))
  (Utilities|Casting|CastToBP_skull OtherActor)
  (bind _asvrpawn (Utilities|Casting|CastToVRPawn (Game|Player|GetPlayerPawn 0)))
  (bind _result (Math|Integer|IncrementInt (Variables|/Game/VRTemplate/Blueprints/VRPawn.VRPawn_C|GetSkullNums _asvrpawn))
    (:%20%20
      (Variables|/Game/VRTemplate/Blueprints/VRPawn.VRPawn_C|SetSkullNums _asvrpawn _result)
      (Variables|Default|SetActive true)
      (CallFunction|ToggleSkullPotColor))))

(event OnComponentEndOverlap(Box)
  (params (OverlappedComponent :type Primitive%20Component%20Object%20Reference) (OtherActor :type Actor%20Object%20Reference) (OtherComp :type Primitive%20Component%20Object%20Reference) (OtherBodyIndex :type Integer))
  (Utilities|Casting|CastToBP_skull OtherActor)
  (bind _asvrpawn (Utilities|Casting|CastToVRPawn (Game|Player|GetPlayerPawn 0)))
  (bind _result (Math|Integer|DecrementInt (Variables|/Game/VRTemplate/Blueprints/VRPawn.VRPawn_C|GetSkullNums _asvrpawn))
    (:%20%20
      (Variables|/Game/VRTemplate/Blueprints/VRPawn.VRPawn_C|SetSkullNums _asvrpawn _result)
      (Variables|Default|SetActive false)
      (CallFunction|ToggleSkullPotColor))))

(event Custom|ToggleSkullPotColor
  (if (Variables|Default|GetActive)
    (Rendering|Components|Light|SetLightColor (Variables|Default|GetPointLight) (Variables|Default|GetActiveColor) false)
    (else
      (Rendering|Components|Light|SetLightColor (Variables|Default|GetPointLight) (Variables|Default|GetNotActiveColor) false))))

(event EventBeginPlay
  (Variables|Default|SetNotActiveColor (Rendering|Components|Light|GetLightColor (Variables|Default|GetPointLight))))

(fn ConstructionScript)